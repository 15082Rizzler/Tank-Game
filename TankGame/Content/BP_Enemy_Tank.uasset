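; Enemy tank Blueprint that chases the player on sight and aims its gun at them.
; PawnSensing triggers an AIMoveTo toward the seen pawn; arrival toggles a Gate that lets Tick smoothly lerp the gun toward it.
; Arrival also runs a debug-drawn line trace from ShootPoint.
; Hitting BP_PlayerTank only clears the ShootingTime flag; no firing is implemented.
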(event OnSeePawn(PawnSensing)
  (params (Pawn :type Pawn%20Object%20Reference))
  (Variables|Default|SetCan%20See%20Player true)
  (CallFunction|ChasePlayer))

(event Custom|Chase%20player
  (bind _shootpoint (Variables|Default|GetShootPoint))
  (bind _returnvalue (Transformation|GetWorldLocation _shootpoint))
  (Variables|Default|SetShooting%20time true)
  (if (Variables|Default|GetCan%20See%20Player)
    (AI|AIMoveTo self "0, 0, 0" (stale OnSeePawn(PawnSensing) Pawn) 5e+02 false
      (:OnSuccess
        (CallFunction|ToggleGate)
        (bind _outhit (Collision|LineTraceByChannel _returnvalue (+ _returnvalue (* (Math|Vector|GetForwardVector (Transformation|GetWorldRotation _shootpoint)) 5e+03)) "TraceTypeQuery1" false 0 "ForDuration" :!label _label))
        (bind _asbp_player_tank (Utilities|Casting|CastToBP_PlayerTank (.HitActor (Collision|BreakHitResult _outhit))))
        (if (== (.HitActor (Collision|BreakHitResult _outhit)) _asbp_player_tank)
          (if (Variables|Default|GetShooting%20time)
            (Variables|Default|SetShooting%20time false))
          (else
            (goto _label)))))
    (else
      (Variables|Default|SetCan%20See%20Player false))))

(event Custom|Toggle%20Gate
  (Utilities|FlowControl|Gate true) ; enters at Toggle
)

(event EventBeginPlay)

(event EventTick
  (params (DeltaSeconds :type Float%20%28single-precision%29))
  (Utilities|FlowControl|Gate true
    (:Exit
      (Transformation|SetWorldRotation (Variables|Default|GetGun) (Math|Rotator|Lerp(Rotator) (Transformation|GetWorldRotation (Variables|Default|GetGun)) (Math|Rotator|FindLookatRotation (Transformation|GetActorLocation self) (Transformation|GetActorLocation (stale OnSeePawn(PawnSensing) Pawn))) 0.25) false false))))

(fn ConstructionScript)