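; BP_MainHUD is the main HUD Blueprint, showing engine status, current gear, shells left and reload state.
; On BeginPlay it creates UI_Widget_1, stores it as UIREF1 and adds it to the viewport.
; Its HUD_ events act as a thin relay, each passing a bool or int straight to the matching update function on that widget.
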(event Custom|HUD_Engine%20check
  (params (Bool%20Input :type Boolean))
  (Default|CheckEngineStatus (Variables|Default|GetUI%20REF%201) Bool%20Input))

(event Custom|HUD_Shells%20left
  (params (Int%20Input :type Integer))
  (Default|CheckShellCount (Variables|Default|GetUI%20REF%201) Int%20Input))

(event Custom|HUD_Reload
  (params (Input%20Bool :type Boolean))
  (Default|CheckReload (Variables|Default|GetUI%20REF%201) Input%20Bool))

(event Custom|HUD_Update%20Gears
  (params (Int%20Input :type Integer))
  (Default|UpdateCurrentGear (Variables|Default|GetUI%20REF%201) Int%20Input))

(event EventBeginPlay
  (bind _returnvalue (UserInterface|CreateWidget "/Game/UI_Widget_1.UI_Widget_1_C"))
  (bind _output_get (Variables|Default|SetUI%20REF%201 _returnvalue))
  (UserInterface|Viewport|AddtoViewport _output_get 0))

(fn ConstructionScript)