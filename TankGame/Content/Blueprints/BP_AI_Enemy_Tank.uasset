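; AI controller for the enemy tank that runs its behavior tree on possess and tracks whether it can see the player.
; AI Perception updates set the CanSeePlayer and Player blackboard keys when an actor tagged Player is sensed.
; Any other perception update starts a line-of-sight timer that clears both keys on expiry, so the tank briefly remembers a lost player.
; Sensing the player again cancels that timer.
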(event OnTargetPerceptionUpdated(AIPerception)
  (params (Actor :type Actor%20Object%20Reference) (Stimulus :type AI%20Stimulus%20Structure))
  (bind _blackboard (Variables|Default|GetBlackboard))
  ;[0.125 0.125 0.125] If the tank sees the player, set can see player to true, and update the blackboard to keep track of the player. If the tank doesn't see the player, clear the reference to the player and set can see player to false
  (if (and (Actor|ActorHasTag Actor "Player") (.bSuccessfullySensed (Utilities|Struct|BreakAIStimulus Stimulus)))
    (Utilities|Time|ClearandInvalidateTimerbyHandle (Variables|Default|GetEnemy%20Timer))
    (AI|Components|Blackboard|SetValueasBool _blackboard (Variables|Default|GetCan%20See%20Player) true)
    (AI|Components|Blackboard|SetValueasObject _blackboard (Variables|Default|GetPlayer) Actor)
    (else
      (bind _returnvalue (Utilities|Time|SetTimerbyEvent (delegate Custom|Start%20Enemy%20Timer) (Variables|Default|GetLine%20Of%20Sight%20Timer)))
      (Variables|Default|SetEnemy%20Timer _returnvalue))))

(event Custom|Start%20Enemy%20Timer
  (bind _blackboard (Variables|Default|GetBlackboard))
  ;[0.125 0.125 0.125] If the tank sees the player, set can see player to true, and update the blackboard to keep track of the player. If the tank doesn't see the player, clear the reference to the player and set can see player to false
  (AI|Components|Blackboard|SetValueasBool _blackboard (Variables|Default|GetCan%20See%20Player) false)
  (AI|Components|Blackboard|SetValueasObject _blackboard (Variables|Default|GetPlayer) 0))

(event EventPossess
  (params (PossessedPawn :type Pawn%20Object%20Reference))
  (AI|RunBehaviorTree "/Game/AI/BT_Enemy_Tank.BT_Enemy_Tank"))

(fn ConstructionScript)