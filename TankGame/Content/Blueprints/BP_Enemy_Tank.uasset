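; BP_Enemy_Tank is an AI tank pawn built to chase and aim at the player tank, feeding roam range to its blackboard on BeginPlay.
; Chaseplayer uses AIMoveTo, then toggles a gate that lets Tick lerp the turret toward the player.
; A forward line trace checks for BP_PlayerTank and clears a shooting flag, but spawns no shot.
; OnSeePawn is empty, leaving the detection and patrol blackboard updates disconnected.
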(event OnSeePawn(PawnSensing)
  (params (Pawn :type Pawn%20Object%20Reference))
  ;[1 0.4951 0.2621] Upon detecting the player, toggle Can See Player, update the blackboard to track the player character and start chasing the player.
)

(event Custom|Chase%20player
  (bind (_outputpin _returnvalue) (CallFunction|FuncShootDIrection))
  (Variables|Default|SetShooting%20time true)
  (if (Variables|Default|GetCan%20See%20Player)
    (AI|AIMoveTo self "0, 0, 0" (stale OnSeePawn(PawnSensing) Pawn) 5e+02 false
      (:OnSuccess
        (CallFunction|ToggleGate)
        (bind _outhit (Collision|LineTraceByChannel _outputpin _returnvalue "TraceTypeQuery1" false 0 "ForDuration" :!label _label))
        (bind _asbp_player_tank (Utilities|Casting|CastToBP_PlayerTank (.HitActor (Collision|BreakHitResult _outhit))))
        (if (== (.HitActor (Collision|BreakHitResult _outhit)) _asbp_player_tank)
          (if (Variables|Default|GetShooting%20time)
            (Variables|Default|SetShooting%20time false))
          (else
            (goto _label)))))
    (else
      (Variables|Default|SetCan%20See%20Player false))))

(event Custom|Toggle%20Gate
  (Utilities|FlowControl|Gate true) ; enters at Toggle
)

(event EventBeginPlay
  (bind (_returnvalue _returnvalue2) (CallFunction|FuncBBData "RoamingRange"))
  ;[1 1 1] Sets up some behaviour tree variables
  (AI|Components|Blackboard|SetValueasFloat _returnvalue _returnvalue2 (Variables|Default|GetMax%20Roam%20Range)))

(event EventTick
  (params (DeltaSeconds :type Float%20%28single-precision%29))
  (Utilities|FlowControl|Gate true
    (:Exit
      (Transformation|SetWorldRotation (Variables|Default|GetGun) (CallFunction|FuncRotateGun (stale OnSeePawn(PawnSensing) Pawn)) false false))))

(fn ConstructionScript)

(fn FuncBBData
  (params (KeyName :type Name))
  ;[1 1 1] Gets the blackboard used by the tank, and allows for a variable in the blackboard to be selected for updating if it's exact name is inputted into key name
  (return (AI|GetBlackboard (AI|GetAIController self)) (Utilities|Name|MakeLiteralName KeyName)))

(fn FuncChangeSpeed
  (params (MoveSpeed :type Float%20%28double-precision%29))
  ;[1 1 1] Changes the speed at which the tank moves at
  (Variables|/Script/Engine.FloatingPawnMovement|SetMaxSpeed (Variables|Default|GetFloatingPawnMovement) MoveSpeed))

(fn FuncShootDIrection
  (bind _shootpoint (Variables|Default|GetShootPoint))
  (bind _returnvalue (Transformation|GetWorldLocation _shootpoint))
  ;[1 1 1] Get the forward vector of shoot point's world rotation, extend it through multiplication, add it to shoot point's world location and output the result. Also output shoot point's world location as a starting point for the line cast.
  (return _returnvalue (+ _returnvalue (* (Math|Vector|GetForwardVector (Transformation|GetWorldRotation _shootpoint)) 5e+03))))

(fn FuncRotateGun
  (params (Detected%20Player :type Actor%20Object%20Reference))
  ;[1 1 1] Rotate the tank's turret by lerping it's rotation between it's world rotaton and the look at rotation between the tank and the player
  (return (Math|Rotator|Lerp(Rotator) (Transformation|GetWorldRotation (Variables|Default|GetGun)) (Math|Rotator|FindLookatRotation (Transformation|GetActorLocation self) (Transformation|GetActorLocation Detected%20Player)) 0.25)))