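; Player-controlled tank pawn with five gears, a toggleable engine, a rotating gun and limited shells, reporting its state to BP_MainHUD.
; Enhanced Input drives FloatingPawnMovement along an Arrow scaled by gear, while turning rotates hull and Arrow and is mutually exclusive with driving.
; Firing spawns BP_Shell and requires a randomly timed manual reload.
; A NoiseRadius component is rescaled by engine state, gear and shots, with firing briefly overriding driving noise.
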(event Input|EnhancedActionEvents|EnhancedInputActionIA_ToggleEngine
  (params (ActionValue :type Boolean) (ElapsedSeconds :type Float%20%28double-precision%29) (TriggeredSeconds :type Float%20%28double-precision%29) (InputAction :type Input%20Action%20Object%20Reference :default "/Game/Input/IA_ToggleEngine.IA_ToggleEngine"))
  (bind _noise_radius (Variables|Default|GetNoise%20Radius))
  (bind _noise_radius_2 (Variables|Default|GetNoise%20Radius))
  ;[0.5604 1 0.7338] Turn engine on/off
  (:Started
    (if (Variables|Default|GetToggle%20engine%20mode)
      (if (Variables|Default|GetToggle%20engine%20mode%202)
        (Variables|Default|SetToggle%20engine%20mode%202 false)
        (Utilities|FlowControl|Delay 1.4)
        (Variables|Default|SetIs%20engine%20on? true)
        (bind _asbp_main_hud (Utilities|Casting|CastToBP_MainHUD (HUD|GetHUD (Game|GetPlayerController 0))))
        (Default|HUDEngineCheck _asbp_main_hud (Variables|Default|GetIs%20engine%20on?))
        (Transformation|SetWorldScale3D _noise_radius (Math|Vector|MakeVector 3.0 3.0 (.z (Transformation|GetWorldScale _noise_radius))))
        (Variables|Default|SetToggle%20engine%20mode false))
      (elif (not (Variables|Default|GetToggle%20engine%20mode%202))
        (Variables|Default|SetToggle%20engine%20mode%202 true)
        (Variables|Default|SetIs%20engine%20on? false)
        (Variables|Default|SetDriving false)
        (Variables|Default|SetTurning false)
        (bind _asbp_main_hud_2 (Utilities|Casting|CastToBP_MainHUD (HUD|GetHUD (Game|GetPlayerController 0))))
        (Default|HUDEngineCheck _asbp_main_hud_2 (Variables|Default|GetIs%20engine%20on?))
        (Transformation|SetWorldScale3D _noise_radius_2 (Math|Vector|MakeVector 0.0 0.0 (.z (Transformation|GetWorldScale _noise_radius_2))))
        (Variables|Default|SetToggle%20engine%20mode true)))))

(event Input|EnhancedActionEvents|EnhancedInputActionIA_MoveUpDown
  (params (ActionValue :type Float%20%28double-precision%29) (ElapsedSeconds :type Float%20%28double-precision%29) (TriggeredSeconds :type Float%20%28double-precision%29) (InputAction :type Input%20Action%20Object%20Reference :default "/Game/Input/IA_MoveUpDown.IA_MoveUpDown"))
  (bind _noise_radius (Variables|Default|GetNoise%20Radius))
  (bind _noise_radius_2 (Variables|Default|GetNoise%20Radius))
  (bind _noise_radius_3 (Variables|Default|GetNoise%20Radius))
  (bind _gear_noise_level (Variables|Default|GetGear%20noise%20level))
  (bind _gear_noise_level_2 (Variables|Default|GetGear%20noise%20level))
  ;[1 0.756 0.1085] Moving
  (:Triggered
    (if (Variables|Default|GetIs%20engine%20on?)
      (if (not (Variables|Default|GetTurning))
        (Variables|Default|SetDriving true)
        (if (> ActionValue 0.0)
          (Class|PawnMovementComponent|AddInputVector (Variables|Default|GetFloatingPawnMovement) (* (Math|Vector|GetForwardVector (Variables|Default|GetArrow)) (* "0.500000,0.500000,0.000000" (Variables|Default|GetGear%20multiplier))) false)
          (if (not (Variables|Default|GetDon't%20emit%20sound%20driving))
            (Transformation|SetWorldScale3D _noise_radius_2 (Math|Vector|MakeVector _gear_noise_level_2 _gear_noise_level_2 (.z (Transformation|GetWorldScale _noise_radius_2)))))
          (else
            (Class|PawnMovementComponent|AddInputVector (Variables|Default|GetFloatingPawnMovement) (* (Math|Vector|RotateVector (Math|Vector|GetForwardVector (Variables|Default|GetArrow)) "0.000000,180.000000,0.000000") (* "0.500000,0.500000,0.000000" (Variables|Default|GetGear%20multiplier))) false)
            (if (not (Variables|Default|GetDon't%20emit%20sound%20driving))
              (Transformation|SetWorldScale3D _noise_radius_3 (Math|Vector|MakeVector _gear_noise_level _gear_noise_level (.z (Transformation|GetWorldScale _noise_radius_3))))))))))
  (:Completed
    (if (Variables|Default|GetIs%20engine%20on?)
      (Variables|Default|SetDriving false)
      (Transformation|SetWorldScale3D _noise_radius (Math|Vector|MakeVector 3.0 3.0 (.z (Transformation|GetWorldScale _noise_radius)))))))

(event Input|EnhancedActionEvents|EnhancedInputActionIA_5thGear
  (params (ActionValue :type Boolean) (ElapsedSeconds :type Float%20%28double-precision%29) (TriggeredSeconds :type Float%20%28double-precision%29) (InputAction :type Input%20Action%20Object%20Reference :default "/Game/Input/IA_5thGear.IA_5thGear"))
  ;[0 0.3218 1] Change gears
  (:Started
    (Variables|Default|SetGear 5)
    (Variables|Default|SetGear%20multiplier "1.600000,1.600000,0.000000")
    (Variables|Default|SetGear%20noise%20level 11.0)
    (bind _asbp_main_hud (Utilities|Casting|CastToBP_MainHUD (HUD|GetHUD (Game|GetPlayerController 0))))
    (Default|HUDUpdateGears _asbp_main_hud (Variables|Default|GetGear))))

(event Input|EnhancedActionEvents|EnhancedInputActionIA_MoveLeftRight
  (params (ActionValue :type Float%20%28double-precision%29) (ElapsedSeconds :type Float%20%28double-precision%29) (TriggeredSeconds :type Float%20%28double-precision%29) (InputAction :type Input%20Action%20Object%20Reference :default "/Game/Input/IA_MoveLeftRight.IA_MoveLeftRight"))
  (bind _arrow (Variables|Default|GetArrow))
  (bind _tank (Variables|Default|GetTank))
  ;[0.4982 0.2768 1] Turning
  (:Triggered
    (if (Variables|Default|GetIs%20engine%20on?)
      (if (not (Variables|Default|GetDriving))
        (Variables|Default|SetTurning true)
        (if (> ActionValue 0.0)
          (Transformation|AddLocalRotation _arrow "0.000000,1.000000,0.000000" false false)
          (Transformation|AddLocalRotation _tank "0.000000,1.000000,0.000000" false false)
          (else
            (Transformation|AddLocalRotation _arrow "0.000000,-1.000000,0.000000" false false)
            (Transformation|AddLocalRotation _tank "0.000000,-1.000000,0.000000" false false))))))
  (:Completed
    (if (Variables|Default|GetIs%20engine%20on?)
      (Variables|Default|SetTurning false))))

(event Input|EnhancedActionEvents|EnhancedInputActionIA_RotateGun
  (params (ActionValue :type Float%20%28double-precision%29) (ElapsedSeconds :type Float%20%28double-precision%29) (TriggeredSeconds :type Float%20%28double-precision%29) (InputAction :type Input%20Action%20Object%20Reference :default "/Game/Input/IA_RotateGun.IA_RotateGun"))
  ;[1 0.3604 0.6837] Rotate Gun
  (if (Variables|Default|GetIs%20engine%20on?)
    (if (> ActionValue 0.0)
      (Transformation|AddLocalRotation (Variables|Default|GetGun) "0.000000,1.000000,0.000000" false false)
      (else
        (Transformation|AddLocalRotation (Variables|Default|GetGun) "0.000000,-1.000000,0.000000" false false)))))

(event Input|EnhancedActionEvents|EnhancedInputActionIA_ShootTank
  (params (ActionValue :type Boolean) (ElapsedSeconds :type Float%20%28double-precision%29) (TriggeredSeconds :type Float%20%28double-precision%29) (InputAction :type Input%20Action%20Object%20Reference :default "/Game/Input/IA_ShootTank.IA_ShootTank"))
  (bind _noise_radius (Variables|Default|GetNoise%20Radius))
  (bind _noise_radius_2 (Variables|Default|GetNoise%20Radius))
  ;[1 0.125 0.125] Shooting
  (:Started
    (Utilities|FlowControl|Sequence
      (:then_0
        (Variables|Default|SetDon't%20emit%20sound%20driving true)
        (Utilities|FlowControl|Delay 0.2)
        (Variables|Default|SetDon't%20emit%20sound%20driving false))
      (:then_1
        (if (Variables|Default|GetIs%20engine%20on?)
          (if (Variables|Default|GetIs%20turret%20loaded?)
            (if (> (Variables|Default|GetShells%20left) 0)
              (Game|SpawnActorfromClass "/Game/Blueprints/BP_Shell.BP_Shell_C" (Math|Transform|MakeTransform (Transformation|GetWorldLocation (Variables|Default|GetShootPoint)) (Transformation|GetWorldRotation (Variables|Default|GetGun)) "1.000000,1.000000,1.000000") "Undefined" "MultiplyWithRoot" 0 0)
              (Variables|Default|SetIs%20turret%20loaded? false)
              (bind _output_get (Variables|Default|SetShells%20left (- (Variables|Default|GetShells%20left) 1)))
              (bind _asbp_main_hud (Utilities|Casting|CastToBP_MainHUD (HUD|GetHUD (Game|GetPlayerController 0))))
              (Default|HUDShellsLeft _asbp_main_hud _output_get)
              (Transformation|SetWorldScale3D _noise_radius_2 (Math|Vector|MakeVector 12.0 12.0 (.z (Transformation|GetWorldScale _noise_radius_2))))
              (if (not (Variables|Default|GetDriving))
                (Utilities|FlowControl|Delay 0.2)
                (Transformation|SetWorldScale3D _noise_radius (Math|Vector|MakeVector 4.0 4.0 (.z (Transformation|GetWorldScale _noise_radius))))))))))))

(event Input|EnhancedActionEvents|EnhancedInputActionIA_Reload
  (params (ActionValue :type Boolean) (ElapsedSeconds :type Float%20%28double-precision%29) (TriggeredSeconds :type Float%20%28double-precision%29) (InputAction :type Input%20Action%20Object%20Reference :default "/Game/Input/IA_Reload.IA_Reload"))
  ;[1 0.3651 0] Reload turret
  (:Started
    (if (not (Variables|Default|GetIs%20turret%20loaded?))
      (bind _asbp_main_hud (Utilities|Casting|CastToBP_MainHUD (HUD|GetHUD (Game|GetPlayerController 0))))
      (Default|HUDReload _asbp_main_hud (Variables|Default|GetIs%20turret%20loaded?))
      (Utilities|FlowControl|Delay (Math|Random|RandomFloatinRange 3.2 6.8))
      (bind _output_get (Variables|Default|SetIs%20turret%20loaded? true))
      (Default|HUDReload _asbp_main_hud _output_get))))

(event Input|EnhancedActionEvents|EnhancedInputActionIA_1stGear
  (params (ActionValue :type Boolean) (ElapsedSeconds :type Float%20%28double-precision%29) (TriggeredSeconds :type Float%20%28double-precision%29) (InputAction :type Input%20Action%20Object%20Reference :default "/Game/Input/IA_1stGear.IA_1stGear"))
  ;[0 0.3218 1] Change gears
  (:Started
    (Variables|Default|SetGear 1)
    (Variables|Default|SetGear%20multiplier "0.400000,0.400000,0.000000")
    (Variables|Default|SetGear%20noise%20level 3.0)
    (bind _asbp_main_hud (Utilities|Casting|CastToBP_MainHUD (HUD|GetHUD (Game|GetPlayerController 0))))
    (Default|HUDUpdateGears _asbp_main_hud (Variables|Default|GetGear))))

(event Input|EnhancedActionEvents|EnhancedInputActionIA_2ndGear
  (params (ActionValue :type Boolean) (ElapsedSeconds :type Float%20%28double-precision%29) (TriggeredSeconds :type Float%20%28double-precision%29) (InputAction :type Input%20Action%20Object%20Reference :default "/Game/Input/IA_2ndGear.IA_2ndGear"))
  ;[0 0.3218 1] Change gears
  (:Started
    (Variables|Default|SetGear 2)
    (Variables|Default|SetGear%20multiplier "0.700000,0.700000,0.000000")
    (Variables|Default|SetGear%20noise%20level 5.0)
    (bind _asbp_main_hud (Utilities|Casting|CastToBP_MainHUD (HUD|GetHUD (Game|GetPlayerController 0))))
    (Default|HUDUpdateGears _asbp_main_hud (Variables|Default|GetGear))))

(event Input|EnhancedActionEvents|EnhancedInputActionIA_3rdGear
  (params (ActionValue :type Boolean) (ElapsedSeconds :type Float%20%28double-precision%29) (TriggeredSeconds :type Float%20%28double-precision%29) (InputAction :type Input%20Action%20Object%20Reference :default "/Game/Input/IA_3rdGear.IA_3rdGear"))
  ;[0 0.3218 1] Change gears
  (:Started
    (Variables|Default|SetGear 3)
    (Variables|Default|SetGear%20multiplier "1.000000,1.000000,0.000000")
    (Variables|Default|SetGear%20noise%20level 7.0)
    (bind _asbp_main_hud (Utilities|Casting|CastToBP_MainHUD (HUD|GetHUD (Game|GetPlayerController 0))))
    (Default|HUDUpdateGears _asbp_main_hud (Variables|Default|GetGear))))

(event Input|EnhancedActionEvents|EnhancedInputActionIA_4thGear
  (params (ActionValue :type Boolean) (ElapsedSeconds :type Float%20%28double-precision%29) (TriggeredSeconds :type Float%20%28double-precision%29) (InputAction :type Input%20Action%20Object%20Reference :default "/Game/Input/IA_4thGear.IA_4thGear"))
  ;[0 0.3218 1] Change gears
  (:Started
    (Variables|Default|SetGear 4)
    (Variables|Default|SetGear%20multiplier "1.300000,1.300000,0.000000")
    (Variables|Default|SetGear%20noise%20level 9.0)
    (bind _asbp_main_hud (Utilities|Casting|CastToBP_MainHUD (HUD|GetHUD (Game|GetPlayerController 0))))
    (Default|HUDUpdateGears _asbp_main_hud (Variables|Default|GetGear))))

(event EventBeginPlay
  ;[1 1 1] BeginPlay
  (Input|AddMappingContext (PlayerController|LocalPlayerSubsystems|GetEnhancedInputLocalPlayerSubsystem (Game|GetPlayerController 0)) "/Game/Input/IMC_Tank.IMC_Tank" 0 "(bIgnoreAllPressedKeysUntilRelease=True,bForceImmediately=False,bNotifyUserSettings=False)")
  (bind _asbp_main_hud (Utilities|Casting|CastToBP_MainHUD (HUD|GetHUD (Game|GetPlayerController 0))))
  (Default|HUDEngineCheck _asbp_main_hud (Variables|Default|GetIs%20engine%20on?))
  (Default|HUDShellsLeft _asbp_main_hud (Variables|Default|GetShells%20left))
  (Default|HUDReload _asbp_main_hud (Variables|Default|GetIs%20turret%20loaded?))
  (Default|HUDUpdateGears _asbp_main_hud (Variables|Default|GetGear)))

(fn ConstructionScript)