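; BP_Shell is a shell actor that travels in a straight line along its Arrow component's forward vector.
; BeginPlay caches the starting location and enables movement.
; Each Tick moves it a fixed horizontal step, with Z zeroed and no delta-time scaling, so speed depends on frame rate.
; It teleports without sweeping and contains no active hit or lifetime logic.
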(event EventBeginPlay
  ;[1 1 1] Get the shell's initial location and allow it to move
  (Variables|Default|SetCurrent%20Location (Transformation|GetActorLocation))
  (Variables|Default|SetReady%20to%20Move true))

(event Collision|EventActorBeginOverlap
  (params (OtherActor :type Actor%20Object%20Reference)))

(event EventTick
  (params (DeltaSeconds :type Float%20%28single-precision%29))
  ;[0.9735 1 0] Travel forward according to this actor's forward vector
  (if (Variables|Default|GetReady%20to%20Move)
    (Transformation|SetActorLocation (+ (* (Math|Vector|GetForwardVector (Variables|Default|GetArrow)) "50.000000,50.000000,0.000000") (Variables|Default|GetCurrent%20Location)) false true)
    (Variables|Default|SetCurrent%20Location (Transformation|GetActorLocation))))

(fn ConstructionScript)