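; AI controller for enemy tanks that runs BT_Enemy_Tank on possession and creates looping-style turret and tread sounds, toggled by events and silenced by the player tank's mute flag.
; AI Perception writes player visibility and reference to the Blackboard, clearing them after a line-of-sight grace delay.
; Reload restores CanFire after a random delay to limit shell spam.
; Hearing radius is settable, but its noise-detection logic is disconnected.
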(event OnTargetPerceptionUpdated(AIPerception)
  (params (Actor :type Actor%20Object%20Reference) (Stimulus :type AI%20Stimulus%20Structure))
  (bind (_varname _blackboard) (CallFunction|FuncAIContData "Can See Player"))
  (bind (_varname_2 _blackboard_2) (CallFunction|FuncAIContData "Player"))
  (bind (_varname_3 _blackboard_3) (CallFunction|FuncAIContData "Can See Player"))
  (bind (_varname_4 _blackboard_4) (CallFunction|FuncAIContData "Player"))
  ;[0.125 0.125 0.125] If the tank sees the player, set can see player to true, and update the blackboard to keep track of the player. If the tank doesn't see the player, clear the reference to the player and set can see player to false
  (if (and (Actor|ActorHasTag Actor "Player") (.bSuccessfullySensed (Utilities|Struct|BreakAIStimulus Stimulus)))
    (Development|PrintString "Player Spotted")
    (Variables|Default|SetCanSeePlayerRefBool true)
    (CallFunction|Testago)
    (AI|Components|Blackboard|SetValueasBool _blackboard _varname true)
    (AI|Components|Blackboard|SetValueasObject _blackboard_2 _varname_2 Actor)
    (else
      (Variables|Default|SetCanSeePlayerRefBool false)
      (Utilities|FlowControl|DoOnce false :!label _label
        (:Completed
          (Utilities|FlowControl|Delay (Variables|Default|GetLine%20Of%20Sight%20Timer))
          (if (Variables|Default|GetCanSeePlayerRefBool)
            (goto _label Reset)
            (else
              (AI|Components|Blackboard|SetValueasBool _blackboard_3 _varname_3 false)
              (AI|Components|Blackboard|SetValueasObject _blackboard_4 _varname_4 0)
              (goto _label Reset))))))))

(event Custom|Reload
  (bind (_varname _blackboard) (CallFunction|FuncAIContData "CanFire"))
  ;[0.7552 0 0.687 0.5] Reload after shooting as to not spam shells at the player
  (Development|PrintString "reloading")
  (Utilities|FlowControl|Delay (Math|Random|RandomFloatinRange 3.2 6.8))
  (AI|Components|Blackboard|SetValueasBool _blackboard _varname true)
  (Development|PrintString "Finished!"))

(event Custom|Change%20Hearing%20Radius
  (params (Noise%20Value :type Float%20%28double-precision%29))
  ;[0.102 0.9403 1 0.5] Change the Hearing Radius. Called by the Player's BP
  (Variables|Default|SetHearing%20Radius Noise%20Value))

(event Custom|Testago
  (Variables|Default|SetTest true)
  (Utilities|FlowControl|Delay 5.0)
  (Variables|Default|SetTest false))

(event Custom|LogPlayer
  (params (Player%20Input :type BP%20Player%20Tank%20Object%20Reference))
  (Utilities|FlowControl|DoOnce false
    (:Completed
      (Variables|Default|SetPlayerRef Player%20Input))))

(event Custom|Noise%20Detection)

(event Custom|SOUND_Rotate%20Turret
  (params (Input :type Boolean))
  (bind _returnvalue (Actor|GetActorOfClass "/Game/Blueprints/BP_PlayerTank.BP_PlayerTank_C"))
  (if (Variables|/Game/Blueprints/BP_PlayerTank.BP_PlayerTank_C|GetMute%20Enemy%20Movement _returnvalue)
    (Components|Activation|SetActive (Variables|Default|GetSOUND_TurretRotation) false false)
    (else
      (Components|Activation|SetActive (Variables|Default|GetSOUND_TurretRotation) Input false))))

(event Custom|SOUND_Rotate%20Treads
  (params (Input :type Boolean))
  (bind _returnvalue (Actor|GetActorOfClass "/Game/Blueprints/BP_PlayerTank.BP_PlayerTank_C"))
  (if (Variables|/Game/Blueprints/BP_PlayerTank.BP_PlayerTank_C|GetMute%20Enemy%20Movement _returnvalue)
    (Components|Activation|SetActive (Variables|Default|GetSOUND_TankTreadsRotating) false false)
    (else
      (Components|Activation|SetActive (Variables|Default|GetSOUND_TankTreadsRotating) Input false))))

(event Custom|SOUND_Move%20Treads
  (params (Input :type Boolean))
  (bind _returnvalue (Actor|GetActorOfClass "/Game/Blueprints/BP_PlayerTank.BP_PlayerTank_C"))
  (if (Variables|/Game/Blueprints/BP_PlayerTank.BP_PlayerTank_C|GetMute%20Enemy%20Movement _returnvalue)
    (Components|Activation|SetActive (Variables|Default|GetSOUND_TankTreadsMoving) false false)
    (else
      (Components|Activation|SetActive (Variables|Default|GetSOUND_TankTreadsMoving) Input false))))

(event EventTick
  (params (DeltaSeconds :type Float%20%28single-precision%29)))

(event EventPossess
  (params (PossessedPawn :type Pawn%20Object%20Reference))
  (Variables|Default|SetPossessed%20Tank PossessedPawn)
  (AI|RunBehaviorTree "/Game/AI/BT_Enemy_Tank.BT_Enemy_Tank")
  (bind _returnvalue (Audio|SpawnSound2D "/Game/Sounds/SW_Tank_Turret_Rotating.SW_Tank_Turret_Rotating" 1.0 1.0 0.0 0 false false))
  (bind _output_get (Variables|Default|SetSOUND_TurretRotation _returnvalue))
  (Components|Activation|SetActive _output_get false false)
  (bind _returnvalue_2 (Audio|SpawnSound2D "/Game/Sounds/SW_Tank_Treads_Rotating.SW_Tank_Treads_Rotating" 1.0 1.0 0.0 0 false false))
  (bind _output_get_2 (Variables|Default|SetSOUND_TankTreadsRotating _returnvalue_2))
  (Components|Activation|SetActive _output_get_2 false false)
  (bind _returnvalue_3 (Audio|SpawnSound2D "/Game/Sounds/SW_Tank_Treads_Moving.SW_Tank_Treads_Moving" 1.0 1.0 0.0 0 false false))
  (bind _output_get_3 (Variables|Default|SetSOUND_TankTreadsMoving _returnvalue_3))
  (Components|Activation|SetActive _output_get_3 false false))

(fn ConstructionScript)

(fn FuncAIContData
  (params (BBVarName :type Name))
  (return (Utilities|Name|MakeLiteralName BBVarName) (AI|GetBlackboard 0)))