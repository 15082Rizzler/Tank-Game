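; Enemy tank pawn driven by an AI controller, which takes damage from player shells and explodes when destroyed.
; Pawn sensing passes the first seen pawn to the blackboard's Player key, while helper functions set movement speed and patrol location.
; Overlapping tagged shells reduce Integrity randomly; at zero it destroys its controller, swaps gun materials and updates the player's score.
; Turret rotation and shot-direction functions are marked deprecated.
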(event OnSeePawn(PawnSensing)
  (params (Pawn :type Pawn%20Object%20Reference))
  (bind (_returnvalue _returnvalue2) (CallFunction|FuncBBData "Player"))
  ;[1 0.4951 0.2621] Upon detecting the player, Send a ref of the player's actor to the enemy's AI blackboard
  (Utilities|FlowControl|DoOnce false
    (:Completed
      (AI|Components|Blackboard|SetValueasObject _returnvalue _returnvalue2 Pawn))))

(event OnComponentBeginOverlap(Box)
  (params (OverlappedComponent :type Primitive%20Component%20Object%20Reference) (OtherActor :type Actor%20Object%20Reference) (OtherComp :type Primitive%20Component%20Object%20Reference) (OtherBodyIndex :type Integer) (bFromSweep :type Boolean) (SweepResult :type Hit%20Result%20Structure%20%28by%20ref%29))
  (if (> (Utilities|Array|FindItem (Variables|/Script/Engine.Actor|GetTags OtherActor) "PlayerShell") -1)
    (bind _output_get (Variables|Default|SetIntegrity (- (Variables|Default|GetIntegrity) (Math|Random|RandomFloatinRange 1.0 3.5))))
    (Niagara|SpawnSystematLocation "/Game/VFX/NS_SmallExplosion.NS_SmallExplosion" (Transformation|GetActorLocation OtherActor))
    (Audio|PlaySoundatLocation "/Game/Sounds/SW_Explosion.SW_Explosion" (Transformation|GetActorLocation OtherActor) "0, 0, 0" 1.0 1.0 0.0 0 0 0 0)
    (Actor|DestroyActor OtherActor)
    (if (<= _output_get 0.0)
      (CallFunction|Perish))))

(event Custom|Perish
  (Variables|Default|SetStopShootingWhenDead true)
  (bind _output_get (Variables|Default|SetDeleteThisAIController (AI|GetAIController self)))
  (Pawn|UnPossess _output_get)
  (Actor|DestroyActor (Variables|Default|GetDeleteThisAIController))
  (Rendering|Material|SetMaterial (Variables|Default|GetGun) 0 "/Game/Materials/MAT_BaseNonMetalic.MAT_BaseNonMetalic")
  (Rendering|Material|SetMaterial (Variables|Default|GetGun%20nozzle) 0 "/Game/Materials/MAT_BaseNonMetalic.MAT_BaseNonMetalic")
  (bind _returnvalue (AddComponent|AddNiagaraComponent false))
  (Class|NiagaraComponent|SetAsset _returnvalue "/Game/VFX/NS_Explosion.NS_Explosion" true)
  (bind _returnvalue_2 (Actor|GetActorOfClass "/Game/Blueprints/BP_PlayerTank.BP_PlayerTank_C"))
  (Default|UpdateScore _returnvalue_2))

(fn ConstructionScript)

(fn FuncBBData
  (params (KeyName :type Name))
  ;[1 1 1] Gets the blackboard used by the tank, and allows for a variable in the blackboard to be selected for updating if it's exact name is inputted into key name
  (return (AI|GetBlackboard (AI|GetAIController self)) (Utilities|Name|MakeLiteralName KeyName)))

(fn FuncChangeSpeed
  (params (MoveSpeed :type Float%20%28double-precision%29))
  ;[1 1 1] Changes the speed at which the tank moves at
  (bind _output_get (Variables|/Script/Engine.FloatingPawnMovement|SetMaxSpeed (Variables|Default|GetFloatingPawnMovement) MoveSpeed))
  (Development|PrintString (Utilities|String|ToString(Float) _output_get)))

(fn DEPRECIATEDFuncShootDIrection
  (bind _shootpoint (Variables|Default|GetShootPoint))
  (bind _returnvalue (Transformation|GetWorldLocation _shootpoint))
  ;[1 1 1] Get the forward vector of shoot point's world rotation, extend it through multiplication, add it to shoot point's world location and output the result. Also output shoot point's world location as a starting point for the line cast.
  (return _returnvalue (+ _returnvalue (* (Math|Vector|GetForwardVector (Transformation|GetWorldRotation _shootpoint)) 5e+03))))

(fn DEPRECIATEDFuncRotateGun
  (params (Detected%20Player :type Actor%20Object%20Reference))
  ;[1 1 1] Rotate the tank's turret by lerping it's rotation between it's world rotaton and the look at rotation between the tank and the player
  (if (Variables|Default|GetCan%20See%20Player)
    (return (Math|Rotator|Lerp(Rotator) (Transformation|GetWorldRotation (Variables|Default|GetGun)) (Math|Rotator|FindLookatRotation (Transformation|GetActorLocation self) (Transformation|GetActorLocation Detected%20Player)) 0.25))
    (else
      (return (Math|Rotator|Lerp(Rotator) (Transformation|GetWorldRotation (Variables|Default|GetGun)) (Math|Rotator|FindLookatRotation (Transformation|GetActorLocation self) (Transformation|GetWorldLocation (Variables|Default|GetArrow))) 0.25)))))

(fn FuncUpdatePatrol
  (params (Vector%20Input :type Vector))
  (Variables|Default|SetPatrolLocation Vector%20Input))