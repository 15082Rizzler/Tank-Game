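; Player tank pawn with Enhanced Input controls for engine, five gears, turret rotation, shooting and timed reload.
; Engine state, gear-based driving and firing set a noise level, pushed to every enemy tank as its hearing radius and drawn as a debug circle.
; Driving and hull turning are mutually exclusive, with toggled looping sounds.
; Enemy shell overlaps reduce integrity until death removes input; BP_MainHUD reflects tank state and score.
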(event OnComponentBeginOverlap(Boxcollider)
  (params (OverlappedComponent :type Primitive%20Component%20Object%20Reference) (OtherActor :type Actor%20Object%20Reference) (OtherComp :type Primitive%20Component%20Object%20Reference) (OtherBodyIndex :type Integer) (bFromSweep :type Boolean) (SweepResult :type Hit%20Result%20Structure%20%28by%20ref%29))
  ;[0.07292 0 0.00694 0.5] Get hurt by enemy shells and Die if integrity is depleated
  (if (> (Utilities|Array|FindItem (Variables|/Script/Engine.Actor|GetTags OtherActor) "EnemyShell") -1)
    (Niagara|SpawnSystematLocation "/Game/VFX/NS_SmallExplosion.NS_SmallExplosion" (Transformation|GetActorLocation OtherActor))
    (Audio|PlaySoundatLocation "/Game/Sounds/SW_Explosion.SW_Explosion" (Transformation|GetActorLocation OtherActor) "0, 0, 0" 1.0 1.0 0.0 0 0 0 0)
    (Actor|DestroyActor OtherActor)
    (bind _output_get (Variables|Default|SetTank%20Integrity (- (Variables|Default|GetTank%20Integrity) 1)))
    (bind _asbp_main_hud (Utilities|Casting|CastToBP_MainHUD (HUD|GetHUD (Game|GetPlayerController 0))))
    (Default|HUDUpdateIntegrityMeter _asbp_main_hud _output_get)
    (if (== (Variables|Default|GetTank%20Integrity) 0)
      (Input|RemoveMappingContext (PlayerController|LocalPlayerSubsystems|GetEnhancedInputLocalPlayerSubsystem (Game|GetPlayerController 0)) "/Game/Input/IMC_Tank.IMC_Tank" "(bIgnoreAllPressedKeysUntilRelease=True,bForceImmediately=False,bNotifyUserSettings=False)")
      (Rendering|Material|SetMaterial (Variables|Default|GetGun) 0 "/Game/Materials/MAT_BaseNonMetalic.MAT_BaseNonMetalic")
      (Rendering|Material|SetMaterial (Variables|Default|GetGun%20nozzle) 0 "/Game/Materials/MAT_BaseNonMetalic.MAT_BaseNonMetalic")
      (bind _returnvalue (AddComponent|AddNiagaraComponent false))
      (Class|NiagaraComponent|SetAsset _returnvalue "/Game/VFX/NS_Explosion.NS_Explosion" true)
      (Variables|/Script/Engine.PlayerController|SetbShowMouseCursor (Game|GetPlayerController 0) true)
      (Default|HUDDeathScreen _asbp_main_hud))))

(event Custom|Update%20Score
  ;[0 0.15 0.01016 0.999] Change the score. Usually called by enemies upon their death.
  (bind _output_get (Variables|Default|SetScore (+ (Variables|Default|GetScore) 1)))
  (bind _asbp_main_hud (Utilities|Casting|CastToBP_MainHUD (HUD|GetHUD (Game|GetPlayerController 0))))
  (Default|HUDSetScore _asbp_main_hud _output_get))

(event Input|EnhancedActionEvents|EnhancedInputActionIA_ToggleEngine
  (params (ActionValue :type Boolean) (ElapsedSeconds :type Float%20%28double-precision%29) (TriggeredSeconds :type Float%20%28double-precision%29) (InputAction :type Input%20Action%20Object%20Reference :default "/Game/Input/IA_ToggleEngine.IA_ToggleEngine"))
  ;[0.5604 1 0.7338] Turn engine on/off
  (:Started
    (if (Variables|MovementVars|GetToggle%20engine%20mode)
      (if (Variables|MovementVars|GetToggle%20engine%20mode%202)
        (Variables|MovementVars|SetToggle%20engine%20mode%202 false)
        (Utilities|FlowControl|Delay 1.4)
        (Variables|MovementVars|SetIs%20engine%20on? true)
        (bind _asbp_main_hud (Utilities|Casting|CastToBP_MainHUD (HUD|GetHUD (Game|GetPlayerController 0))))
        (Default|HUDEngineCheck _asbp_main_hud (Variables|MovementVars|GetIs%20engine%20on?))
        (bind _output_get (Variables|NoiseVars|SetNoise%20Level (Variables|NoiseVars|GetEngine%20Passive%20Noise)))
        (CallFunction|FuncUpdateNoise _output_get)
        (Variables|MovementVars|SetToggle%20engine%20mode false))
      (elif (not (Variables|MovementVars|GetToggle%20engine%20mode%202))
        (Variables|MovementVars|SetToggle%20engine%20mode%202 true)
        (Variables|MovementVars|SetIs%20engine%20on? false)
        (Variables|MovementVars|SetDriving false)
        (Variables|MovementVars|SetTurning false)
        (bind _asbp_main_hud_2 (Utilities|Casting|CastToBP_MainHUD (HUD|GetHUD (Game|GetPlayerController 0))))
        (Default|HUDEngineCheck _asbp_main_hud_2 (Variables|MovementVars|GetIs%20engine%20on?))
        (bind _output_get_2 (Variables|NoiseVars|SetNoise%20Level 0.1))
        (CallFunction|FuncUpdateNoise _output_get_2)
        (Variables|MovementVars|SetToggle%20engine%20mode true)))))

(event Input|EnhancedActionEvents|EnhancedInputActionIA_MoveUpDown
  (params (ActionValue :type Float%20%28double-precision%29) (ElapsedSeconds :type Float%20%28double-precision%29) (TriggeredSeconds :type Float%20%28double-precision%29) (InputAction :type Input%20Action%20Object%20Reference :default "/Game/Input/IA_MoveUpDown.IA_MoveUpDown"))
  (bind _sound_tanktreadsmoving (Variables|Default|GetSOUND_TankTreadsMoving))
  ;[1 0.756 0.1085] Moving
  (:Triggered
    (if (Variables|MovementVars|GetIs%20engine%20on?)
      (if (not (Variables|MovementVars|GetTurning))
        (Variables|MovementVars|SetDriving true)
        (if (> ActionValue 0.0)
          (Class|PawnMovementComponent|AddInputVector (Variables|Default|GetFloatingPawnMovement) (* (Math|Vector|GetForwardVector (Variables|Default|GetArrow)) (* "0.500000,0.500000,0.000000" (Variables|MovementVars|GetGear%20multiplier))) false)
          (Components|Activation|SetActive _sound_tanktreadsmoving true false)
          (else
            (Class|PawnMovementComponent|AddInputVector (Variables|Default|GetFloatingPawnMovement) (* (Math|Vector|RotateVector (Math|Vector|GetForwardVector (Variables|Default|GetArrow)) "0.000000,180.000000,0.000000") (* "0.500000,0.500000,0.000000" (Variables|MovementVars|GetGear%20multiplier))) false)
            (Components|Activation|SetActive _sound_tanktreadsmoving true false))))))
  (:Started
    (CallFunction|FuncMoveNoise ActionValue))
  (:Completed
    (Components|Activation|SetActive (Variables|Default|GetSOUND_TankTreadsMoving) false false)
    (if (Variables|MovementVars|GetIs%20engine%20on?)
      (Variables|MovementVars|SetDriving false)
      (bind _output_get (Variables|NoiseVars|SetNoise%20Level (Variables|NoiseVars|GetEngine%20Passive%20Noise)))
      (CallFunction|FuncUpdateNoise _output_get))))

(event Input|EnhancedActionEvents|EnhancedInputActionIA_5thGear
  (params (ActionValue :type Boolean) (ElapsedSeconds :type Float%20%28double-precision%29) (TriggeredSeconds :type Float%20%28double-precision%29) (InputAction :type Input%20Action%20Object%20Reference :default "/Game/Input/IA_5thGear.IA_5thGear"))
  ;[0 0.3218 1] Change gears
  (:Started
    (Variables|MovementVars|SetGear 5)
    (Variables|MovementVars|SetGear%20multiplier "1.600000,1.600000,0.000000")
    (bind _output_get (Variables|NoiseVars|SetGear%20Noise%20Modifier 5.5e+02))
    (CallFunction|FuncUpdateNoise _output_get)
    (bind _asbp_main_hud (Utilities|Casting|CastToBP_MainHUD (HUD|GetHUD (Game|GetPlayerController 0))))
    (Default|HUDUpdateGears _asbp_main_hud (Variables|MovementVars|GetGear))))

(event Input|EnhancedActionEvents|EnhancedInputActionIA_MuteEnemyMovement
  (params (ActionValue :type Boolean) (ElapsedSeconds :type Float%20%28double-precision%29) (TriggeredSeconds :type Float%20%28double-precision%29) (InputAction :type Input%20Action%20Object%20Reference :default "/Game/Input/IA_MuteEnemyMovement.IA_MuteEnemyMovement"))
  ;[0.15 0.15 0.15 0.5] Mute Enemy Movement
  (:Started
    (Utilities|FlowControl|FlipFlop
      (:A
        (Variables|Default|SetMute%20Enemy%20Movement true))
      (:B
        (Variables|Default|SetMute%20Enemy%20Movement false)))))

(event Input|EnhancedActionEvents|EnhancedInputActionIA_MoveLeftRight
  (params (ActionValue :type Float%20%28double-precision%29) (ElapsedSeconds :type Float%20%28double-precision%29) (TriggeredSeconds :type Float%20%28double-precision%29) (InputAction :type Input%20Action%20Object%20Reference :default "/Game/Input/IA_MoveLeftRight.IA_MoveLeftRight"))
  (bind _sound_tanktreadsrotating (Variables|Default|GetSOUND_TankTreadsRotating))
  (bind _arrow (Variables|Default|GetArrow))
  (bind _tank (Variables|Default|GetTank))
  ;[0.4982 0.2768 1] Turning
  (:Triggered
    (if (Variables|MovementVars|GetIs%20engine%20on?)
      (if (not (Variables|MovementVars|GetDriving))
        (Variables|MovementVars|SetTurning true)
        (if (> ActionValue 0.0)
          (Transformation|AddLocalRotation _arrow "0.000000,1.000000,0.000000" false false)
          (Transformation|AddLocalRotation _tank "0.000000,1.000000,0.000000" false false)
          (Components|Activation|SetActive _sound_tanktreadsrotating true false)
          (else
            (Transformation|AddLocalRotation _arrow "0.000000,-1.000000,0.000000" false false)
            (Transformation|AddLocalRotation _tank "0.000000,-1.000000,0.000000" false false)
            (Components|Activation|SetActive _sound_tanktreadsrotating true false))))))
  (:Completed
    (Components|Activation|SetActive (Variables|Default|GetSOUND_TankTreadsRotating) false false)
    (if (Variables|MovementVars|GetIs%20engine%20on?)
      (Variables|MovementVars|SetTurning false))))

(event Input|EnhancedActionEvents|EnhancedInputActionIA_RotateGun
  (params (ActionValue :type Float%20%28double-precision%29) (ElapsedSeconds :type Float%20%28double-precision%29) (TriggeredSeconds :type Float%20%28double-precision%29) (InputAction :type Input%20Action%20Object%20Reference :default "/Game/Input/IA_RotateGun.IA_RotateGun"))
  (bind _sound_turretrotation (Variables|Default|GetSOUND_TurretRotation))
  ;[1 0.3604 0.6837] Rotate Gun
  (:Triggered
    (if (Variables|MovementVars|GetIs%20engine%20on?)
      (if (> ActionValue 0.0)
        (Transformation|AddLocalRotation (Variables|Default|GetGun) "0.000000,1.000000,0.000000" false false)
        (Components|Activation|SetActive _sound_turretrotation true false)
        (else
          (Transformation|AddLocalRotation (Variables|Default|GetGun) "0.000000,-1.000000,0.000000" false false)
          (Components|Activation|SetActive _sound_turretrotation true false)))))
  (:Completed
    (Components|Activation|SetActive (Variables|Default|GetSOUND_TurretRotation) false false)))

(event Input|EnhancedActionEvents|EnhancedInputActionIA_ShootTank
  (params (ActionValue :type Boolean) (ElapsedSeconds :type Float%20%28double-precision%29) (TriggeredSeconds :type Float%20%28double-precision%29) (InputAction :type Input%20Action%20Object%20Reference :default "/Game/Input/IA_ShootTank.IA_ShootTank"))
  ;[1 0.125 0.125] Shooting
  (:Started
    (Utilities|FlowControl|Sequence
      (:then_0
        (Variables|MovementVars|SetDon't%20emit%20sound%20driving true)
        (Utilities|FlowControl|Delay 0.2)
        (Variables|MovementVars|SetDon't%20emit%20sound%20driving false))
      (:then_1
        (if (Variables|MovementVars|GetIs%20engine%20on?)
          (if (Variables|ShootingVars|GetIs%20turret%20loaded?)
            (if (> (Variables|ShootingVars|GetShells%20left) 0)
              (Game|SpawnActorfromClass "/Game/Blueprints/BP_Shell.BP_Shell_C" (Math|Transform|MakeTransform (Transformation|GetWorldLocation (Variables|Default|GetShootPoint)) (Transformation|GetWorldRotation (Variables|Default|GetGun)) "1.000000,1.000000,1.000000") "Undefined" "MultiplyWithRoot" 0 0)
              (Variables|ShootingVars|SetIs%20turret%20loaded? false)
              (bind _output_get (Variables|ShootingVars|SetShells%20left (- (Variables|ShootingVars|GetShells%20left) 1)))
              (bind _asbp_main_hud (Utilities|Casting|CastToBP_MainHUD (HUD|GetHUD (Game|GetPlayerController 0))))
              (Default|HUDShellsLeft _asbp_main_hud _output_get)
              (Variables|ShootingVars|SetJust%20Fired true)
              (bind _output_get_2 (Variables|NoiseVars|SetNoise%20Level 1.05e+03))
              (Audio|PlaySoundatLocation "/Game/Sounds/SW_Tank_Shot.SW_Tank_Shot" (Transformation|GetActorLocation) "0, 0, 0" 1.0 1.0 0.0 0 0 0 0)
              (CallFunction|FuncUpdateNoise _output_get_2)
              (if (Variables|MovementVars|GetDriving)
                (Utilities|FlowControl|Delay 0.2)
                (Variables|NoiseVars|SetNoise%20Level (Variables|NoiseVars|GetGear%20Noise%20Modifier))
                (Variables|ShootingVars|SetJust%20Fired false)
                (else
                  (Utilities|FlowControl|Delay 0.2)
                  (Variables|NoiseVars|SetNoise%20Level (Variables|NoiseVars|GetEngine%20Passive%20Noise))
                  (Variables|ShootingVars|SetJust%20Fired false))))))))))

(event Input|EnhancedActionEvents|EnhancedInputActionIA_Reload
  (params (ActionValue :type Boolean) (ElapsedSeconds :type Float%20%28double-precision%29) (TriggeredSeconds :type Float%20%28double-precision%29) (InputAction :type Input%20Action%20Object%20Reference :default "/Game/Input/IA_Reload.IA_Reload"))
  ;[1 0.3651 0] Reload turret
  (:Started
    (if (not (Variables|ShootingVars|GetIs%20turret%20loaded?))
      (bind _asbp_main_hud (Utilities|Casting|CastToBP_MainHUD (HUD|GetHUD (Game|GetPlayerController 0))))
      (Default|HUDReload _asbp_main_hud (Variables|ShootingVars|GetIs%20turret%20loaded?))
      (Utilities|FlowControl|Delay (Math|Random|RandomFloatinRange 3.2 6.8))
      (bind _output_get (Variables|ShootingVars|SetIs%20turret%20loaded? true))
      (Default|HUDReload _asbp_main_hud _output_get))))

(event Input|EnhancedActionEvents|EnhancedInputActionIA_1stGear
  (params (ActionValue :type Boolean) (ElapsedSeconds :type Float%20%28double-precision%29) (TriggeredSeconds :type Float%20%28double-precision%29) (InputAction :type Input%20Action%20Object%20Reference :default "/Game/Input/IA_1stGear.IA_1stGear"))
  ;[0 0.3218 1] Change gears
  (:Started
    (Variables|MovementVars|SetGear 1)
    (Variables|MovementVars|SetGear%20multiplier "0.400000,0.400000,0.000000")
    (bind _output_get (Variables|NoiseVars|SetGear%20Noise%20Modifier 1.5e+02))
    (CallFunction|FuncUpdateNoise _output_get)
    (bind _asbp_main_hud (Utilities|Casting|CastToBP_MainHUD (HUD|GetHUD (Game|GetPlayerController 0))))
    (Default|HUDUpdateGears _asbp_main_hud (Variables|MovementVars|GetGear))))

(event Input|EnhancedActionEvents|EnhancedInputActionIA_2ndGear
  (params (ActionValue :type Boolean) (ElapsedSeconds :type Float%20%28double-precision%29) (TriggeredSeconds :type Float%20%28double-precision%29) (InputAction :type Input%20Action%20Object%20Reference :default "/Game/Input/IA_2ndGear.IA_2ndGear"))
  ;[0 0.3218 1] Change gears
  (:Started
    (Variables|MovementVars|SetGear 2)
    (Variables|MovementVars|SetGear%20multiplier "0.700000,0.700000,0.000000")
    (bind _output_get (Variables|NoiseVars|SetGear%20Noise%20Modifier 2.5e+02))
    (CallFunction|FuncUpdateNoise _output_get)
    (bind _asbp_main_hud (Utilities|Casting|CastToBP_MainHUD (HUD|GetHUD (Game|GetPlayerController 0))))
    (Default|HUDUpdateGears _asbp_main_hud (Variables|MovementVars|GetGear))))

(event Input|EnhancedActionEvents|EnhancedInputActionIA_3rdGear
  (params (ActionValue :type Boolean) (ElapsedSeconds :type Float%20%28double-precision%29) (TriggeredSeconds :type Float%20%28double-precision%29) (InputAction :type Input%20Action%20Object%20Reference :default "/Game/Input/IA_3rdGear.IA_3rdGear"))
  ;[0 0.3218 1] Change gears
  (:Started
    (Variables|MovementVars|SetGear 3)
    (Variables|MovementVars|SetGear%20multiplier "1.000000,1.000000,0.000000")
    (bind _output_get (Variables|NoiseVars|SetGear%20Noise%20Modifier 3.5e+02))
    (CallFunction|FuncUpdateNoise _output_get)
    (bind _asbp_main_hud (Utilities|Casting|CastToBP_MainHUD (HUD|GetHUD (Game|GetPlayerController 0))))
    (Default|HUDUpdateGears _asbp_main_hud (Variables|MovementVars|GetGear))))

(event Input|EnhancedActionEvents|EnhancedInputActionIA_4thGear
  (params (ActionValue :type Boolean) (ElapsedSeconds :type Float%20%28double-precision%29) (TriggeredSeconds :type Float%20%28double-precision%29) (InputAction :type Input%20Action%20Object%20Reference :default "/Game/Input/IA_4thGear.IA_4thGear"))
  ;[0 0.3218 1] Change gears
  (:Started
    (Variables|MovementVars|SetGear 4)
    (Variables|MovementVars|SetGear%20multiplier "1.300000,1.300000,0.000000")
    (bind _output_get (Variables|NoiseVars|SetGear%20Noise%20Modifier 4.5e+02))
    (CallFunction|FuncUpdateNoise _output_get)
    (bind _asbp_main_hud (Utilities|Casting|CastToBP_MainHUD (HUD|GetHUD (Game|GetPlayerController 0))))
    (Default|HUDUpdateGears _asbp_main_hud (Variables|MovementVars|GetGear))))

(event EventBeginPlay
  ;[1 1 1] BeginPlay
  (Input|AddMappingContext (PlayerController|LocalPlayerSubsystems|GetEnhancedInputLocalPlayerSubsystem (Game|GetPlayerController 0)) "/Game/Input/IMC_Tank.IMC_Tank" 0 "(bIgnoreAllPressedKeysUntilRelease=True,bForceImmediately=False,bNotifyUserSettings=False)")
  (CallFunction|FuncCreateSounds)
  (bind _asbp_main_hud (Utilities|Casting|CastToBP_MainHUD (HUD|GetHUD (Game|GetPlayerController 0))))
  (Default|HUDEngineCheck _asbp_main_hud (Variables|MovementVars|GetIs%20engine%20on?))
  (Default|HUDShellsLeft _asbp_main_hud (Variables|ShootingVars|GetShells%20left))
  (Default|HUDReload _asbp_main_hud (Variables|ShootingVars|GetIs%20turret%20loaded?))
  (Default|HUDUpdateGears _asbp_main_hud (Variables|MovementVars|GetGear))
  (Default|HUDUpdateIntegrityMeter _asbp_main_hud (Variables|Default|GetTank%20Integrity))
  (Default|HUDSetScore _asbp_main_hud (Variables|Default|GetScore))
  (bind _returnvalue (Actor|GetActorOfClass "/Game/Blueprints/BP_PlayerRefBroadcaster.BP_PlayerRefBroadcaster_C"))
  (Default|SetupRefBroadcast _returnvalue self))

(event EventTick
  (params (DeltaSeconds :type Float%20%28single-precision%29))
  (bind _returnvalue (Transformation|GetActorLocation))
  ;[0.15 0.15 0.15 0.5] Debug Noise radius creator
  (Rendering|Debug|DrawDebugCircle (Math|Vector|MakeVector (.x _returnvalue) (.y _returnvalue) (+ (.z _returnvalue) 1e+01)) (Variables|NoiseVars|GetNoise%20Level) 12 "(R=0.319498,G=1.000000,B=0.000000,A=1.000000)" 0.0 1.0 "0.000000,1.000000,0.000000" "1.000000,0.000000,0.000000" true))

(fn ConstructionScript)

(fn FuncUpdateNoise
  (params (Noise%20Input :type Float%20%28double-precision%29))
  (bind _outactors (Actor|GetAllActorsOfClass "/Game/Blueprints/BP_AI_Enemy_Tank.BP_AI_Enemy_Tank_C"))
  (for _array_element _outactors
    (Default|ChangeHearingRadius _array_element Noise%20Input)))

(fn FuncMoveNoise
  (params (Action%20Value :type Float%20%28double-precision%29))
  (if (> Action%20Value 0.0)
    (if (not (Variables|MovementVars|GetDon't%20emit%20sound%20driving))
      (if (not (Variables|ShootingVars|GetJust%20Fired))
        (bind _output_get (Variables|NoiseVars|SetNoise%20Level (Variables|NoiseVars|GetGear%20Noise%20Modifier)))
        (CallFunction|FuncUpdateNoise _output_get)))
    (elif (not (Variables|MovementVars|GetDon't%20emit%20sound%20driving))
      (if (not (Variables|ShootingVars|GetJust%20Fired))
        (bind _output_get_2 (Variables|NoiseVars|SetNoise%20Level (Variables|NoiseVars|GetGear%20Noise%20Modifier)))
        (CallFunction|FuncUpdateNoise _output_get_2)))))

(fn FuncCreateSounds
  (bind _returnvalue (Audio|SpawnSound2D "/Game/Sounds/SW_Tank_Turret_Rotating.SW_Tank_Turret_Rotating" 1.0 1.0 0.0 0 false false))
  (bind _output_get (Variables|Default|SetSOUND_TurretRotation _returnvalue))
  (Components|Activation|SetActive _output_get false false)
  (bind _returnvalue_2 (Audio|SpawnSound2D "/Game/Sounds/SW_Tank_Treads_Rotating.SW_Tank_Treads_Rotating" 1.0 1.0 0.0 0 false false))
  (bind _output_get_2 (Variables|Default|SetSOUND_TankTreadsRotating _returnvalue_2))
  (Components|Activation|SetActive _output_get_2 false false)
  (bind _returnvalue_3 (Audio|SpawnSound2D "/Game/Sounds/SW_Tank_Treads_Moving.SW_Tank_Treads_Moving" 1.0 1.0 0.0 0 false false))
  (bind _output_get_3 (Variables|Default|SetSOUND_TankTreadsMoving _returnvalue_3))
  (Components|Activation|SetActive _output_get_3 false false))