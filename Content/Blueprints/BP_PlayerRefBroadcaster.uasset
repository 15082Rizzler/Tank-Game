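; BP_PlayerRefBroadcaster hands a player actor reference to every BP_AI_Enemy_Tank in the level.
; SetupRefBroadcast stores the passed-in player, starts the broadcast and prints a debug string.
; BroadcastToEnemies finds all tanks by class, sets each one's PlayerRef and calls its LogPlayer.
; The event then re-calls itself after a long delay, repeating the broadcast indefinitely instead of using Tick.
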(event Custom|SetupRefBroadcast
  (params (PlayerRef :type BP%20Player%20Tank%20Object%20Reference))
  (Variables|Default|SetPlayer%20Actor PlayerRef)
  (CallFunction|BroadcasttoEnemies)
  (Development|PrintString "Fired Off"))

(event Custom|BroadcastToEnemies
  (bind _outactors (Actor|GetAllActorsOfClass "/Game/Blueprints/BP_AI_Enemy_Tank.BP_AI_Enemy_Tank_C"))
  (for _array_element _outactors
    (Variables|/Game/Blueprints/BP_AI_Enemy_Tank.BP_AI_Enemy_Tank_C|SetPlayerRef _array_element (Variables|Default|GetPlayer%20Actor))
    (Default|LogPlayer _array_element))
  (Utilities|FlowControl|Delay 2e+01)
  (CallFunction|BroadcasttoEnemies))

(event EventBeginPlay)

(event Collision|EventActorBeginOverlap
  (params (OtherActor :type Actor%20Object%20Reference)))

(event EventTick
  (params (DeltaSeconds :type Float%20%28single-precision%29)))

(fn ConstructionScript)